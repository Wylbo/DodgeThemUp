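; Player-controlled sci-fi fighter ship that moves, banks, dodges sideways and fires twin cannons.
; Axis inputs drive yaw-relative planar movement, while four timelines play and reverse to tilt Box1, their outputs summed into one rotation.
; Dodge timelines spin the ship mesh and force movement along world Y, with CanDodge blocking further dodges and firing until finished.
; Tick runs Shoot, which spawns BP_Shoot from both cannons at a timed interval while Space is held.
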(event EventTick
  (params (DeltaSeconds :type Float%20%28single-precision%29))
  ;[1 1 1] Shoot
  (CallFunction|Shoot DeltaSeconds))

(event Input|ActionEvents|InputActionDodgeLeft
  (params (Key :type Key%20Structure :default "None"))
  ;[1 1 1] Dodge
  (:Pressed
    (if (Variables|Default|GetcanDodge)
      (Variables|Default|SetcanDodge false)
      (bind _rotation (Timeline|DodgeLeft PlayFromStart)
        (:Update
          (Transformation|SetRelativeRotation (Variables|Default|GetSM_SciFi_Fighter) (Math|Rotator|MakeRotator 0.0 _rotation -9e+01) false false)
          (Pawn|Input|AddMovementInput "0,-1.000000, 0" (Variables|Default|GetdodgeDistance) true))
        (:Finished
          (Variables|Default|SetcanDodge true))))))

(event Input|ActionEvents|InputActionDodgeRight
  (params (Key :type Key%20Structure :default "None"))
  ;[1 1 1] Dodge
  (:Pressed
    (if (Variables|Default|GetcanDodge)
      (Variables|Default|SetcanDodge false)
      (bind _rotation (Timeline|DodgeRight PlayFromStart)
        (:Update
          (Transformation|SetRelativeRotation (Variables|Default|GetSM_SciFi_Fighter) (Math|Rotator|MakeRotator 0.0 _rotation -9e+01) false false)
          (Pawn|Input|AddMovementInput "0,1.000000, 0" (Variables|Default|GetdodgeDistance) true))
        (:Finished
          (Variables|Default|SetcanDodge true))))))

(event Input|AxisEvents|InputAxisMoveForward
  (params (AxisValue :type Float%20%28single-precision%29))
  (bind _returnvalue (Input|AxisValues|GetMoveForward))
  ;[1 1 1] Movement
  ;;[0.3177 0.9128 1] Forward Backward
  (Pawn|Input|AddMovementInput (Math|Vector|GetForwardVector (Math|Rotator|MakeRotator 0.0 0.0 (.Yaw (Math|Rotator|BreakRotator (Pawn|GetControlRotation :!class /Script/Engine.Pawn))))) AxisValue false)
  ;;[0.4538 1 0.6823] Tilt
  (if (> _returnvalue 0.0)
    (Variables|Default|SetisGoingForward true)
    (bind _forward (Timeline|Tilt%20forward Play)
      (:Update
        (Transformation|SetRelativeRotation (Variables|Default|GetBox1) (Math|Rotator|MakeRotator (+ (stale Input|AxisEvents|InputAxisMoveRight _angle) (stale Input|AxisEvents|InputAxisMoveRight _angle_2)) (+ _forward (stale _backward)) 0.0) false false :!label _label)))
    (elif (< _returnvalue 0.0)
      (Variables|Default|SetisGoingForward false)
      (bind _backward (Timeline|TiltBack Play)
        (:Update
          (goto _label)))
      (elif (Variables|Default|GetisGoingForward)
        (Variables|Default|SetisGoingForward false)
        (Timeline|Tilt%20forward Reverse)
        (else
          (Timeline|TiltBack Reverse))))))

(event Input|AxisEvents|InputAxisMoveRight
  (params (AxisValue :type Float%20%28single-precision%29))
  (bind _returnvalue (Input|AxisValues|GetMoveRight))
  ;[1 1 1] Movement
  ;;[0.3177 0.9128 1] Right Left
  (Pawn|Input|AddMovementInput (Math|Vector|GetRightVector (Math|Rotator|MakeRotator 0.0 0.0 (.Yaw (Math|Rotator|BreakRotator (Pawn|GetControlRotation :!class /Script/Engine.Pawn))))) AxisValue false)
  ;;[0.4538 1 0.6823] Tilt
  (if (> _returnvalue 0.0)
    (Variables|Default|SetisGoingRight true)
    (bind _angle (Timeline|Tilt%20right Play)
      (:Update
        (Transformation|SetRelativeRotation (Variables|Default|GetBox1) (Math|Rotator|MakeRotator (+ _angle (stale _angle_2)) (+ (stale Input|AxisEvents|InputAxisMoveForward _forward) (stale Input|AxisEvents|InputAxisMoveForward _backward)) 0.0) false false :!label _label)))
    (elif (< _returnvalue 0.0)
      (Variables|Default|SetisGoingRight false)
      (bind _angle_2 (Timeline|TiltLeft Play)
        (:Update
          (goto _label)))
      (elif (Variables|Default|GetisGoingRight)
        (Variables|Default|SetisGoingRight false)
        (Timeline|Tilt%20right Reverse)
        (else
          (Timeline|TiltLeft Reverse))))))

(fn ConstructionScript)

(fn Shoot
  (params (DeltaTime :type Float%20%28single-precision%29))
  (bind _output_get (Variables|Default|SetTimer (+ DeltaTime (Variables|Default|GetTimer))))
  (if (Math|Boolean|ANDBoolean (>= _output_get (Variables|Default|GetTimeBtwShoot)) (Game|Player|IsInputKeyDown (Game|GetPlayerController 0) "SpaceBar") (Variables|Default|GetcanDodge))
    (Variables|Default|SetTimer 0.0)
    (Utilities|FlowControl|Sequence
      (:then_0
        (Game|SpawnActorfromClass "/Game/BluePrint/BP_Shoot.BP_Shoot_C" (Math|Transform|MakeTransform (Transformation|GetWorldLocation (Variables|Default|GetCanon%201)) (Math|Rotator|MakeRotator 0.0 0.0 0.0)) "Undefined" 0 0))
      (:then_1
        (Game|SpawnActorfromClass "/Game/BluePrint/BP_Shoot.BP_Shoot_C" (Math|Transform|MakeTransform (Transformation|GetWorldLocation (Variables|Default|GetCanon%202)) (Math|Rotator|MakeRotator 0.0 0.0 0.0)) "Undefined" 0 0)))))