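; Player Blueprint that moves on the XY plane from MoveForward and MoveRight axis input.
; On BeginPlay it caches BP_GameMode, then a timeline slides it along +X while spinning its roll, setting MovementEnabled when finished.
; Tick applies the input-driven speeds as a swept per-frame offset, without delta-time scaling or a MovementEnabled check.
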(event EventBeginPlay
  ;[1 1 1] Spawn animation
  (bind _asbp_game_mode (Utilities|Casting|CastToBP_GameMode (Game|GetGameMode)))
  (Variables|Default|SetGameMode _asbp_game_mode)
  (Variables|Default|Setroll (.Roll (Math|Rotator|BreakRotator (Transformation|GetActorRotation))))
  (Variables|Default|SetspawnPosition (Transformation|GetActorLocation))
  (bind _speed (Timeline|Spawn%20Animation Play)
    (:Update
      (Transformation|SetActorLocation (Math|Vector|Lerp(Vector) (Variables|Default|GetspawnPosition) (+ (Variables|Default|GetspawnPosition) "60.000000, 0, 0") _speed) false false)
      (Transformation|SetActorRotation (Math|Rotator|Lerp(Rotator) "0, 0, 0" (Math|Rotator|MakeRotator (+ (Variables|Default|Getroll) (Variables|Default|GetSpawnSpin)) 0.0 0.0) _speed)))
    (:Finished
      (Variables|Default|SetmovementEnabled true))))

(event EventTick
  (params (DeltaSeconds :type Float%20%28single-precision%29))
  (Variables|Default|SetdeltaSecond DeltaSeconds)
  (Transformation|SetActorLocation (+ (Transformation|GetActorLocation) (Math|Vector|MakeVector (Variables|Default|GetvertSpeed) (Variables|Default|GethoriSpeed) 0.0)) true false))

(event Input|AxisEvents|InputAxisMoveRight
  (params (AxisValue :type Float%20%28single-precision%29))
  (Variables|Default|SethoriSpeed (* AxisValue (Variables|Default|GetmovementSpeed))))

(event Input|AxisEvents|InputAxisMoveForward
  (params (AxisValue :type Float%20%28single-precision%29))
  (Variables|Default|SetvertSpeed (* AxisValue (Variables|Default|GetmovementSpeed))))

(fn ConstructionScript)