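; BP_EnemyProjectileBase is the base enemy projectile, which damages the player on hit.
; Construction applies scale and speed and creates a dynamic material instance, which BeginPlay tints with the projectile colour.
; A mesh hit on a damageable player applies damage and explodes with particle and sound calls before destroying the actor.
; Hits on a non-damageable player destroy it silently, while any other hit explodes without damage.
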(event OnComponentHit(StaticMesh)
  (params (HitComponent :type Primitive%20Component%20Object%20Reference) (OtherActor :type Actor%20Object%20Reference) (OtherComp :type Primitive%20Component%20Object%20Reference) (NormalImpulse :type Vector :default "0, 0, 0") (Hit :type Hit%20Result%20Structure%20%28by%20ref%29))
  (bind _asbp_player (Utilities|Casting|CastToBP_Player OtherActor)
    (:then
      (bind _output_get (Variables|Default|SetBP_Player _asbp_player))
      (if (Variables|/Game/BluePrint/BP_Player.BP_Player_C|GetCanTakeDamage _output_get)
        (Game|Damage|ApplyDamage (Variables|Default|GetBP_Player) (Variables|Default|GetDamage) 0 0)
        (CallFunction|Explose :!label _label)
        (else
          (Actor|DestroyActor))))
    (:CastFailed
      (goto _label))))

(event EventBeginPlay
  (Rendering|Material|SetVectorParameterValue (Variables|Default|GetPrjectile%20mat) "Colour" (Variables|Default|GetProjectileColor) :!class /Script/Engine.MaterialInstanceDynamic))

(fn ConstructionScript
  (bind _projectilemovement (Variables|Default|GetProjectileMovement))
  (bind _returnvalue (Rendering|Material|CreateDynamicMaterialInstance (Variables|Default|GetStaticMesh) 0 0 "None" :!class /Script/Engine.PrimitiveComponent))
  (Variables|Default|SetPrjectile%20mat _returnvalue)
  (Transformation|SetWorldScale3D (Variables|Default|GetStaticMesh) (Variables|Default|GetScale))
  (bind _output_get (Variables|/Script/Engine.ProjectileMovementComponent|SetMaxSpeed _projectilemovement (Variables|Default|GetSpeed)))
  (Variables|/Script/Engine.ProjectileMovementComponent|SetInitialSpeed _projectilemovement _output_get))

(fn Explose
  (bind _returnvalue (Transformation|GetActorLocation))
  (Effects|SpawnEmitteratLocation "/Game/StarterContent/Particles/P_Explosion.P_Explosion" _returnvalue)
  (Audio|PlaySoundatLocation 0 _returnvalue "0, 0, 0" 1.0 1.0 0.0 0 0 0)
  (Actor|DestroyActor))