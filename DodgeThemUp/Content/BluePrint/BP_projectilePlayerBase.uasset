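; BP_projectilePlayerBase is a base player projectile with configurable colour, mesh scale and speed.
; The construction script creates a dynamic material on the static mesh, applies the scale, and uses MaxSpeed as both the initial and maximum speed of its ProjectileMovement.
; On BeginPlay it writes the colour to the material's "Colour" parameter.
; It contains no hit or damage logic in these graphs.
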(event EventBeginPlay
  (Rendering|Material|SetVectorParameterValue (Variables|Default|GetProjectileMat) "Colour" (Variables|Default|GetColor) :!class /Script/Engine.MaterialInstanceDynamic))

(fn ConstructionScript
  (bind _projectilemovement (Variables|Default|GetProjectileMovement))
  (bind _returnvalue (Rendering|Material|CreateDynamicMaterialInstance (Variables|Default|GetStaticMesh) 0 0 "None" :!class /Script/Engine.PrimitiveComponent))
  (Variables|Default|SetProjectileMat _returnvalue)
  (Transformation|SetWorldScale3D (Variables|Default|GetStaticMesh) (Variables|Default|GetScale))
  (bind _output_get (Variables|/Script/Engine.ProjectileMovementComponent|SetMaxSpeed _projectilemovement (Variables|Default|GetmaxSpeed)))
  (Variables|/Script/Engine.ProjectileMovementComponent|SetInitialSpeed _projectilemovement _output_get))