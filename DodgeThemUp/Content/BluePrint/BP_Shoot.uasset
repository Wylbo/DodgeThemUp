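; BP_Shoot is a self-moving, short-lived actor that, going by its name, serves as a fired shot.
; Each Tick adds a world transform offset along its forward vector, scaled by Speed but not by DeltaSeconds, so travel speed depends on frame rate.
; It also accumulates ElapsedTime and destroys itself once LifeTime is reached, with no sweep or hit handling in its graphs.
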(event EventTick
  (params (DeltaSeconds :type Float%20%28single-precision%29))
  (Class|Actor|AddActorWorldTransform (Math|Transform|MakeTransform (* (Transformation|GetActorForwardVector) (Variables|Default|Getspeed)) "0, 0, 0" "100.000000,1,1") false false)
  (bind _output_get (Variables|Default|SetelapsedTime (+ (Variables|Default|GetelapsedTime) DeltaSeconds)))
  (if (>= _output_get (Variables|Default|GetlifeTime))
    (Actor|DestroyActor)))

(fn ConstructionScript)