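; BP_GameMode is the game mode that tracks score, top score and enemy counts, creates the HUD, and shows the game-over widget with UI-only input.
; It also wraps world camera shakes and runs timed global time dilation, optionally keeping the player at normal speed via inverse custom dilation.
; The delay is scaled by the dilation to last real seconds, then calls OnEndTimeDilation.
; LoadScore and SaveScore are empty stubs.
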(event Custom|EventChangeTimeDilation
  (params (TimeScale :type Float%20%28single-precision%29) (time :type Float%20%28single-precision%29) (PlayerScale :type Boolean))
  (bind _bp_player (Variables|Default|GetBP_Player))
  (Utilities|Time|SetGlobalTimeDilation TimeScale)
  (if PlayerScale
    (Variables|/Script/Engine.Actor|SetCustomTimeDilation _bp_player (/ 1.0 TimeScale)))
  (Utilities|FlowControl|Delay (* time TimeScale))
  (bind _output_get (Variables|/Script/Engine.Actor|SetCustomTimeDilation _bp_player 1.0))
  (Utilities|Time|SetGlobalTimeDilation _output_get)
  (Default|CallOnEndTimeDilation))

(event EventBeginPlay
  (Development|ExecuteConsoleCommand "r.MotionBlur.TargetFPS 0" 0)
  (Utilities|FlowControl|Sequence
    (:then_0
      (bind _asbp_player (Utilities|Casting|CastToBP_Player (Game|Player|GetPlayerPawn 0)))
      (Variables|Default|SetBP_Player _asbp_player))
    (:then_1
      (Input|SetInputModeGameOnly (Game|GetPlayerController 0))
      (CallFunction|LoadScore)
      (CallFunction|SetScore)
      (bind _returnvalue (UserInterface|CreateWidget "/Game/BluePrint/BPW_HUD.BPW_HUD_C"))
      (bind _output_get (Variables|Default|SetBPW_HUD _returnvalue))
      (UserInterface|Viewport|AddtoViewport _output_get 0))))

(event EventEndPlay
  (params (EndPlayReason :type EEndPlayReason%20Enum :default "Destroyed"))
  (CallFunction|SaveScore))

(fn ConstructionScript)

(fn LoadScore)

(fn SaveScore)

(fn SetScore
  (params (val :type Integer))
  (bind _output_get (Variables|Default|SetScore (+ val (Variables|Default|GetScore))))
  (if (>= _output_get (Variables|Default|GetTopScore))
    (Variables|Default|SetTopScore (Variables|Default|GetScore))
    (else
      (Variables|Default|SetTopScore (Variables|Default|GetTopScore)))))

(fn UpdateEnemyCount
  (params (val :type Integer))
  (Variables|Default|SetEnemiesCount (+ val (Variables|Default|GetEnemiesCount))))

(fn PlayCameraShake
  (params (Shake :type Camera%20Shake%20Class%20Reference) (Epicenter :type Vector))
  (Camera|PlayWorldCameraShake Shake Epicenter 0.0 0.0))

(fn GameOver
  (bind _returnvalue (Game|GetPlayerController 0))
  (bind _returnvalue_2 (UserInterface|CreateWidget "/Game/BluePrint/BPW_GameOver.BPW_GameOver_C"))
  (UserInterface|Viewport|AddtoViewport _returnvalue_2 0)
  (Variables|/Script/Engine.PlayerController|SetbShowMouseCursor _returnvalue false)
  (Input|SetInputModeUIOnly _returnvalue 0 "DoNotLock"))

(fn EnemyKilled
  (Math|Integer|IncrementInt (Variables|Default|GetEnemiesKilled)
    (:%20%20
      (CallFunction|UpdateEnemyCount -1))))

(fn SetGlobalTimeDilation
  (params (TimeDilation :type Float%20%28single-precision%29))
  (Utilities|Time|SetGlobalTimeDilation TimeDilation))