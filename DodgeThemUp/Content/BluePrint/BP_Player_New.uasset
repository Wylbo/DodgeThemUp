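; Player pawn for a shooter on the X-Z plane, with timer-driven firing, dodging, health and a power meter.
; Tick applies interpolated input speeds as swept moves with banking, and wall hits bounce them.
; Dodging teleports along velocity; near enemies or their projectiles it triggers brief slow motion and charges power.
; Full power slows global time while compensating the player's dilation and fire rate; death plays timeline-driven time and camera effects.
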(event OnComponentHit(Box)
  (params (HitComponent :type Primitive%20Component%20Object%20Reference) (OtherActor :type Actor%20Object%20Reference) (OtherComp :type Primitive%20Component%20Object%20Reference) (NormalImpulse :type Vector :default "0, 0, 0") (Hit :type Hit%20Result%20Structure%20%28by%20ref%29))
  (bind (_x _y _z) (Math|Vector|BreakVector (.normal Hit)))
  (bind _bouncefactor (Variables|Default|GetBounceFactor))
  ;[1 1 1] Bounce on wall hit
  (Variables|Default|SethoriSpeed (* (* (Math|Float|Absolute(Float) (Variables|Default|GethoriSpeed)) _bouncefactor) _x))
  (Variables|Default|SetvertSpeed (* _z (* (Math|Float|Absolute(Float) (Variables|Default|GetvertSpeed)) _bouncefactor))))

(event Custom|PrimFire
  ;[1 1 1] Shoot
  (CallFunction|PrimaryFire (Transformation|GetWorldTransform (Variables|Default|GetShootSpawn))))

(event Custom|ResetMat
  (Rendering|Material|SetMaterial (Variables|Default|GetStaticMesh) 0 "/Game/Assets/Materials/Glow/M_GlowPlayer1.M_GlowPlayer1")
  (Variables|Default|SetmovementEnabled true))

(event EventBeginPlay
  ;[1 1 1] Spawn animation
  (bind _asbp_game_mode (Utilities|Casting|CastToBP_GameMode (Game|GetGameMode)))
  (Variables|Default|SetGameMode _asbp_game_mode)
  (Variables|Default|Setroll (.Roll (Math|Rotator|BreakRotator (Transformation|GetActorRotation))))
  (Variables|Default|SetspawnPosition (Transformation|GetActorLocation))
  (bind _speed (Timeline|Spawn%20Animation Play)
    (:Update
      (Transformation|SetActorLocation (Math|Vector|Lerp(Vector) (Variables|Default|GetspawnPosition) (+ (Variables|Default|GetspawnPosition) "0.000000,0.000000,60.000000") _speed) false false)
      (Transformation|SetRelativeRotation (Variables|Default|GetStaticMesh) (Math|Rotator|Lerp(Rotator) "0, 0, 0" (Math|Rotator|MakeRotator 0.0 0.0 (+ (Variables|Default|Getroll) (Variables|Default|GetSpawnSpin))) _speed) false false))
    (:Finished
      (Variables|Default|SetmovementEnabled true))))

(event Game|Damage|EventAnyDamage
  (params (Damage :type Float%20%28single-precision%29) (DamageType :type Damage%20Type%20Object%20Reference) (InstigatedBy :type Controller%20Object%20Reference) (DamageCauser :type Actor%20Object%20Reference))
  (bind _returnvalue (Transformation|GetActorLocation))
  (bind _gamemode (Variables|Default|GetGameMode))
  (bind _springarm (Variables|Default|GetSpringArm))
  ;[1 1 1] Take damage
  (if (Variables|Default|GetCanTakeDamage)
    (bind _output_get (Variables|Default|SetcurrentHp (Math|Float|Clamp(Float) (- (Variables|Default|GetcurrentHp) Damage) 0.0 (Variables|Default|GetMaxHp))))
    (if (<= _output_get 0.0)
      (Effects|SpawnEmitteratLocation 0 _returnvalue)
      (Audio|PlaySoundatLocation 0 _returnvalue "0, 0, 0" 1.0 1.0 0.0 0 0 0)
      (Default|PlayCameraShake _gamemode 0 _returnvalue)
      (Default|GameOver _gamemode)
      (Utilities|FlowControl|Sequence
        (:then_0
          (Variables|Default|SetCanTakeDamage false)
          (Utilities|FlowControl|Sequence
            (:then_0
              (bind _timescale (Timeline|timescale Play)
                (:Update
                  (Utilities|Time|SetGlobalTimeDilation _timescale)
                  (Variables|Default|SetCustomTimeDilation (/ 1.0 _timescale)))))
            (:then_1
              (bind (_direction _springarmlenght _socketoffsett) (Timeline|Death_SpringArm Play)
                (:Update
                  (Variables|/Script/Engine.SpringArmComponent|SetTargetArmLength _springarm _springarmlenght)
                  (Variables|/Script/Engine.SpringArmComponent|SetSocketOffset _springarm (Math|Vector|MakeVector 0.0 _socketoffsett 0.0)))
                (:Finished
                  (Niagara|SpawnSystematLocation "/Game/Assets/Particles/Niagara/Player/NS_Death.NS_Death" (Transformation|GetActorLocation)))))))
        (:then_1
          (Variables|Default|SetmovementSpeed 0.0))))))

(event EventTick
  (params (DeltaSeconds :type Float%20%28single-precision%29))
  (bind _staticmesh (Variables|Default|GetStaticMesh))
  ;[1 1 1] Movement
  (Variables|Default|SetdeltaSecond DeltaSeconds)
  (Transformation|SetActorLocation (+ (Transformation|GetActorLocation) (Math|Vector|MakeVector (Variables|Default|GethoriSpeed) 0.0 0.0)) true false)
  (Transformation|SetActorLocation (+ (Transformation|GetActorLocation) (Math|Vector|MakeVector 0.0 0.0 (Variables|Default|GetvertSpeed))) true false)
  (Transformation|SetRelativeRotation _staticmesh (Class|KismetMathLibrary|RInterptoConstant (Variables|/Script/Engine.SceneComponent|GetRelativeRotation _staticmesh) (Math|Rotator|MakeRotator 0.0 0.0 (+ (* (Variables|Default|GethoriSpeed) (Variables|Default|GetrollFactor)) (Variables|Default|Getroll))) (Variables|Default|GetdeltaSecond) (Variables|Default|GetrollSpeed)) false false))

(event Input|ActionEvents|InputActionDodge
  (params (Key :type Key%20Structure :default "None"))
  ;[1 1 1] Dodge
  (:Pressed
    (CallFunction|Dodge)
    (Utilities|FlowControl|Sequence
      (:then_0
        ;;[0.2807 0.88 1] Invinsible CD
        (Utilities|FlowControl|Delay (Variables|Default|GetInvisible%20Time))
        (Variables|Default|SetCanTakeDamage true)
        (Variables|Default|SetmovementEnabled true)
        (Collision|SetCollisionEnabled (Variables|Default|GetStaticMesh) "QueryAndPhysics"))
      (:then_1
        ;;[0.4002 1 0.7968] Dodge Cooldown
        (Variables|Default|SetCanDodge false)
        (Utilities|FlowControl|Delay (Variables|Default|GetDodgeCD))
        (Variables|Default|SetCanDodge true)))))

(event Input|ActionEvents|InputActionActivatePower
  (params (Key :type Key%20Structure :default "None"))
  (bind _timedilatationfactor (Variables|Default|GettimeDilatationFactor))
  ;[1 1 1] Power
  (:Pressed
    (if (>= (Variables|Default|GetCurrentPower) (Variables|Default|GetMaxPower))
      (Variables|Default|SetCurrentPower 0.0)
      (Rendering|SetVisibility (Variables|Default|GetNiagara) true false)
      (Utilities|FlowControl|Sequence
        (:then_0
          (Variables|Default|SetCanStackPower false)
          (Utilities|FlowControl|Delay (Variables|Default|GetSuperTime))
          (Rendering|SetVisibility (Variables|Default|GetNiagara) false false)
          (Variables|Default|SetCanStackPower true)
          (bind _output_get (Variables|Default|SetCustomTimeDilation 1.0))
          (Utilities|Time|SetGlobalTimeDilation _output_get)
          (Variables|Default|SetFireRate (* (Variables|Default|GetFireRate) (Variables|Default|GettimeDilatationFactor))))
        (:then_1
          (Utilities|Time|SetGlobalTimeDilation (/ 1.0 _timedilatationfactor))
          (Variables|Default|SetCustomTimeDilation _timedilatationfactor)
          (Variables|Default|SetFireRate (/ (Variables|Default|GetFireRate) _timedilatationfactor))
          (Default|CallChangeTimeDilation))))))

(event Input|ActionEvents|InputActionShoot
  (params (Key :type Key%20Structure :default "None"))
  ;[1 1 1] Shoot
  (:Pressed
    (if (Variables|Default|GetmovementEnabled)
      (Utilities|Time|SetTimerbyFunctionName 0 "PrimFire" (Variables|Default|GetFireRate) true)
      (CallFunction|PrimaryFire (Transformation|GetWorldTransform (Variables|Default|GetShootSpawn)))))
  (:Released
    (Utilities|Time|ClearTimerbyFunctionName 0 "PrimFire")))

(event Input|AxisEvents|InputAxisMoveRight
  (params (AxisValue :type Float%20%28single-precision%29))
  ;[1 1 1] Player input
  (bind _directionspeed (CallFunction|Movement (Variables|Default|GethoriSpeed) AxisValue))
  (Variables|Default|SethoriSpeed _directionspeed))

(event Input|AxisEvents|InputAxisMoveForward
  (params (AxisValue :type Float%20%28single-precision%29))
  ;[1 1 1] Player input
  (bind _directionspeed (CallFunction|Movement (Variables|Default|GetvertSpeed) AxisValue))
  (Variables|Default|SetvertSpeed _directionspeed))

(event Input|KeyboardEvents|AnyKey
  (params (Key :type Key%20Structure :default "None"))
  (:Pressed
    (EventDispatchers|BindEventtoOnEndTimeDilation (Variables|Default|GetGameMode) (delegate Custom|ResetMat))))

(fn ConstructionScript
  (Variables|Default|SetcurrentHp (Variables|Default|GetMaxHp))
  (Variables|Default|SetCurrentPower 0.0))

(fn Movement
  (params (speed :type Float%20%28single-precision%29) (Direction :type Float%20%28single-precision%29))
  (return (Math|Interpolation|FInterpTo speed (* Direction (Variables|Default|GetmovementSpeed)) (Variables|Default|GetdeltaSecond) 6.0)))

(fn PrimaryFire
  (params (SpawnTransform :type Transform))
  (Game|SpawnActorfromClass "/Game/BluePrint/Projectile/BP_projectilePlayerBase_Primiry.BP_projectilePlayerBase_Primiry_C" SpawnTransform "AlwaysSpawn" 0 (LocalVariables|GetColor) self))

(fn Dodge
  (bind _staticmesh (Variables|Default|GetStaticMesh))
  (bind _returnvalue (Transformation|GetWorldTransform _staticmesh))
  (if (Variables|Default|GetCanDodge)
    (CallFunction|TestDodgePower)
    (Collision|SetCollisionEnabled (Variables|Default|GetStaticMesh) "NoCollision")
    (bind _output_get (LocalVariables|SetDodgeDirection (Math|Vector|MakeVector (Math|Float|Clamp(Float) (Variables|Default|GethoriSpeed) -1.0) 0.0 (Math|Float|Clamp(Float) (Variables|Default|GetvertSpeed) -1.0))))
    (Niagara|SpawnSystematLocation "/Game/Assets/Particles/Niagara/Dodge/NS_Dodge.NS_Dodge" (.location _returnvalue) (.rotation _returnvalue))
    (Transformation|SetActorLocation (+ (Transformation|GetActorLocation) (* (Math|Vector|Normalize _output_get) (Variables|Default|GetDodgeDistance))) true true)
    (Variables|Default|SetCanDodge false)
    (Variables|Default|SetmovementEnabled false)
    (Default|PlayCameraShake (Variables|Default|GetGameMode) "/Game/BluePrint/BP_ScreenShake.BP_ScreenShake_C" (Transformation|GetActorLocation))))

(fn TestDodgePower
  (bind _dodgeboosttrigger (Variables|Default|GetDodgeBoostTrigger))
  (bind _staticmesh (Variables|Default|GetStaticMesh))
  (if (Variables|Default|GetCanStackPower)
    (for _array_element (Collision|GetOverlappingActors _dodgeboosttrigger 0 :!class /Script/Engine.PrimitiveComponent)
      (bind _asbp_enemy_projectile_base (Utilities|Casting|CastToBP_EnemyProjectileBase _array_element)
        (:then
          _)
        (:CastFailed
          (bind _asbp_enemy_base (Utilities|Casting|CastToBP_EnemyBase _array_element))))
      (if (or (Collision|IsOverlappingActor _dodgeboosttrigger _asbp_enemy_base :!class /Script/Engine.PrimitiveComponent) (Collision|IsOverlappingActor _dodgeboosttrigger _asbp_enemy_projectile_base :!class /Script/Engine.PrimitiveComponent))
        (bind _result (Math|Float|IncrementFloat (Variables|Default|GetCurrentPower))
          (:%20%20
            (Default|EventChangeTimeDilation (Variables|Default|GetGameMode) 0.05 0.5 false)
            (Variables|Default|SetmovementEnabled false)
            (Niagara|SpawnSystemAttached "/Game/Assets/Particles/Niagara/Dodge/Ns_PerfectDodge.NS_PerfectDodge" _staticmesh "None" "0, 0, 0" "0, 0, 0" "KeepRelativeOffset" true)
            (Rendering|Material|SetMaterial _staticmesh 0 "/Game/Assets/Materials/Glow/M_GlowPlayerPerfectDodge.M_GlowPlayerPerfectDodge")
            (Variables|Default|SetCanTakeDamage false)))))))

(fn Death)