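; Spawner actor that drops asteroids, and has logic for enemies, at random X/Y points within its collision bounds at its own Z.
; BeginPlay loops a timer into SpawnAsteroid, whose Delay inside the random-count loop absorbs overlapping triggers.
; SpawnEnemy caps BP_Enemy1 by GameMode count and adds BP_Enemy2 on every fifth kill, but its timer is disconnected here.
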(event Custom|SpawnEnemy
  (bind _bp_gamemode (Variables|Default|GetBP_GameMode))
  (bind _enemieskilled (Variables|/Game/BluePrint/GameMode/BP_GameMode.BP_GameMode_C|GetEnemiesKilled _bp_gamemode))
  (if (< (Variables|/Game/BluePrint/GameMode/BP_GameMode.BP_GameMode_C|GetEnemiesCount _bp_gamemode) (Variables|/Game/BluePrint/GameMode/BP_GameMode.BP_GameMode_C|GetMaxEnemies _bp_gamemode))
    (if (and (== (Math|Integer|%(Integer) _enemieskilled 5) 0) (!= _enemieskilled (Variables|Default|GetCurrentEnemiesKilled)))
      (CallFunction|SpawnEnemy2))
    (Utilities|FlowControl|Delay (Math|Random|RandomFloatinRange 0.5 2.0))
    (Game|SpawnActorfromClass "/Game/BluePrint/Enemies/BP_Enemy1.BP_Enemy1_C" (Math|Transform|MakeTransform (CallFunction|GetRandomLocation) "0, 0, 0" "1,1,1") "Undefined" 0 0)))

(event Custom|SpawnEnemy2
  (Variables|Default|SetCurrentEnemiesKilled (Variables|/Game/BluePrint/GameMode/BP_GameMode.BP_GameMode_C|GetEnemiesKilled (Variables|Default|GetBP_GameMode)))
  (Game|SpawnActorfromClass "/Game/BluePrint/Enemies/BP_Enemy2.BP_Enemy2_C" (Math|Transform|MakeTransform (CallFunction|GetRandomLocation) "0, 0, 0" "1,1,1") "Undefined" 0 0))

(event Custom|SpawnAsteroid
  (for _index (range 0 (Math|Random|RandomIntegerinRange 1 3))
    (Utilities|FlowControl|Delay (Math|Random|RandomFloatinRange 0.5 3.0))
    (Game|SpawnActorfromClass "/Game/BluePrint/Enemies/BP_Asteroid.BP_Asteroid_C" (Math|Transform|MakeTransform (CallFunction|GetRandomLocation) "0, 0, 0" "1,1,1") "Undefined" 0 0)))

(event EventBeginPlay
  (bind _asbp_game_mode (Utilities|Casting|CastToBP_GameMode (Game|GetGameMode)))
  (Variables|Default|SetBP_GameMode _asbp_game_mode)
  (Utilities|FlowControl|Sequence
    (:then_1
      (Utilities|Time|SetTimerbyFunctionName 0 "SpawnAsteroid" 1.0 true))))

(fn ConstructionScript)

(fn GetRandomLocation
  (bind _collisioncomponent (Variables|Default|GetCollisionComponent))
  (bind (_origin _boxextent) (Collision|GetComponentBounds _collisioncomponent))
  (bind _returnvalue (Math|Random|RandomPointinBoundingBox _origin _boxextent))
  (return (Math|Vector|MakeVector (.x _returnvalue) (.y _returnvalue) (.z (Transformation|GetActorLocation)))))