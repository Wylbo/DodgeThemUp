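; Base enemy Blueprint that descends on a spawn timeline, then slides along X at random speed and direction.
; Tick drives swept movement and a delay-throttled FireNode, which spawns projectiles when the player is within X range.
; Non-projectile hits reverse direction, and player collisions damage the player and kill the enemy.
; Death from collision or lost HP triggers effects and reports score, kill and camera shake to BP_GameMode.
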(event EventBeginPlay
  ;[1 1 1] Setup ref and var
  (bind _asbp_game_mode (Utilities|Casting|CastToBP_GameMode (Game|GetGameMode)))
  (bind _output_get (Variables|Default|SetBP_GameMode _asbp_game_mode))
  (Default|UpdateEnemyCount _output_get 1)
  (Variables|Default|SetMoveDirection (Math|Random|RandomBool))
  (Variables|Default|SetMoveSpeed (Math|Random|RandomFloatinRange (Variables|Default|GetMinSpeed) (Variables|Default|GetMaxSpeed)))
  (Variables|Default|SetSpawnLocation (Transformation|GetActorLocation))
  ;[1 1 1] Spawn animation
  (bind _entry_speed (Timeline|Spawn%20animation Play)
    (:Update
      (Transformation|SetActorLocation (Math|Vector|Lerp(Vector) (Variables|Default|GetSpawnLocation) (- (Variables|Default|GetSpawnLocation) "0.000000,0.000000,60.000000") _entry_speed) false false))
    (:Finished
      (Variables|Default|SetMoveEnable true))))

(event Game|Damage|EventAnyDamage
  (params (Damage :type Float%20%28single-precision%29) (DamageType :type Damage%20Type%20Object%20Reference) (InstigatedBy :type Controller%20Object%20Reference) (DamageCauser :type Actor%20Object%20Reference))
  ;[1 1 1] Take damage + Death
  (bind _output_get (Variables|Default|SetHp (Math|Float|Clamp(Float) (- (Variables|Default|GetHp) Damage) 0.0 (Variables|Default|GetMaxHp))))
  (if (<= _output_get 0.0)
    (CallFunction|EnemyKilled)))

(event EventTick
  (params (DeltaSeconds :type Float%20%28single-precision%29))
  ;[1 1 1] Basic movement
  (if (Variables|Default|GetMoveEnable)
    (Transformation|SetActorLocation (+ (Transformation|GetActorLocation) (* (Math|Vector|MakeVector (* (Variables|Default|GetMoveSpeed) (Math|Float|SelectFloat 1.0 -1.0 (Variables|Default|GetMoveDirection))) 0.0 0.0) DeltaSeconds)) true false)
    (|FireNode)))

(event Collision|EventHit
  (params (MyComp :type Primitive%20Component%20Object%20Reference) (Other :type Actor%20Object%20Reference) (OtherComp :type Primitive%20Component%20Object%20Reference) (bSelfMoved :type Boolean) (HitLocation :type Vector :default "0, 0, 0") (HitNormal :type Vector :default "0, 0, 0") (NormalImpulse :type Vector :default "0, 0, 0") (Hit :type Hit%20Result%20Structure%20%28by%20ref%29))
  ;[1 1 1] Switch dir on wall hit or one shot by player collision
  (Utilities|Casting|CastToBP_ProjectilePlayerBase Other
    (:CastFailed
      (Variables|Default|SetMoveDirection (not (Variables|Default|GetMoveDirection)))
      (bind _asbp_player (Utilities|Casting|CastToBP_Player Other))
      (Game|Damage|ApplyDamage _asbp_player 5e+01 0 0)
      (CallFunction|EnemyKilled))))

(fn ConstructionScript)

(fn EnemyKilled
  (bind _returnvalue (Transformation|GetActorLocation))
  (bind _bp_gamemode (Variables|Default|GetBP_GameMode))
  (Effects|SpawnEmitteratLocation "/Game/Assets/Pixel/P_Pixel_Explosion_Enemy.P_Pixel_Explosion_Enemy" (Transformation|GetActorLocation))
  (Default|EnemyKilled _bp_gamemode)
  (Default|SetScore _bp_gamemode (Variables|Default|GetEnemy%20score))
  (Default|PlayCameraShake _bp_gamemode 0 _returnvalue)
  (Audio|PlaySoundatLocation 0 _returnvalue "0, 0, 0" 1.0 1.0 0.0 0 0 0)
  (Actor|DestroyActor))