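; BP_Abyss is an enemy actor that takes damage from BP_Shoot projectiles and is destroyed when its health runs out.
; The construction script sets current HP to max HP.
; On Box component hit by a BP_Shoot, it prints a debug "Hello", subtracts the shot's truncated damage from current HP, and destroys itself at zero or below.
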(event OnComponentHit(Box)
  (params (HitComponent :type Primitive%20Component%20Object%20Reference) (OtherActor :type Actor%20Object%20Reference) (OtherComp :type Primitive%20Component%20Object%20Reference) (NormalImpulse :type Vector :default "0, 0, 0") (Hit :type Hit%20Result%20Structure%20%28by%20ref%29))
  (bind _asbp_shoot (Utilities|Casting|CastToBP_Shoot OtherActor))
  (Development|PrintString "Hello")
  (bind _output_get (Variables|Default|SetcurrentHp (- (Variables|Default|GetcurrentHp) (Math|Float|Truncate (Variables|/Game/BluePrint/BP_Shoot.BP_Shoot_C|Getdamage _asbp_shoot)))))
  (if (<= _output_get 0)
    (Actor|DestroyActor)))

(fn ConstructionScript
  (Variables|Default|SetcurrentHp (Variables|Default|GetmaxHp)))