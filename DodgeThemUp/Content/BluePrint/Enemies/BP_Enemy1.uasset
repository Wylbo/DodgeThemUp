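; BP_Enemy1 is an enemy Blueprint, apparently unfinished, with a mode intended for seeking out the player.
; BeginPlay casts and caches player pawn 0 as a BP_Player.
; In the Search Player mode, Tick sets a target location from the player's Box position plus an offset.
; The static mesh is then set to the world origin, as the computed target is not fed into that move.
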(event EventBeginPlay
  (|CallParentFunction)
  (bind _asbp_player (Utilities|Casting|CastToBP_Player (Game|Player|GetPlayerPawn 0)))
  (Variables|Default|SetBP_Player _asbp_player))

(event EventTick
  (params (DeltaSeconds :type Float%20%28single-precision%29))
  (switch Utilities|FlowControl|Switch|SwitchonE_Enemy2Modes (Variables|Default|GetModes)
    (:NewEnumerator1
      (Variables|Default|SetTargetLocation (+ (Variables|Default|GetTargetOffset) (Transformation|GetWorldLocation (Variables|/Game/BluePrint/BP_Player.BP_Player_C|GetBox (Variables|Default|GetBP_Player)))))
      (Transformation|SetWorldLocation (Variables|Default|GetStaticMesh) "0, 0, 0" false false))))

(fn ConstructionScript
  (|CallParentFunction))