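; Asteroid enemy that moves by ProjectileMovement and takes the player's mesh as its homing target on BeginPlay.
; The construction script applies its scale and rolls a random speed within a range, used as both initial and max speed.
; Any hit on its mesh calls EnemyKilled, which passes its score to BP_GameMode, triggers a camera shake and sound there, then destroys the actor.
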(event OnComponentHit(StaticMesh)
  (params (HitComponent :type Primitive%20Component%20Object%20Reference) (OtherActor :type Actor%20Object%20Reference) (OtherComp :type Primitive%20Component%20Object%20Reference) (NormalImpulse :type Vector :default "0, 0, 0") (Hit :type Hit%20Result%20Structure%20%28by%20ref%29))
  (CallFunction|EnemyKilled))

(event EventBeginPlay
  (bind _returnvalue (Game|Player|GetPlayerPawn 0))
  (bind _asbp_game_mode (Utilities|Casting|CastToBP_GameMode (Game|GetGameMode)))
  (Variables|Default|SetBP_GameMode _asbp_game_mode)
  (Utilities|IsValid _returnvalue
    (:Is%20Valid
      (bind _asbp_player (Utilities|Casting|CastToBP_Player _returnvalue))
      (Variables|/Script/Engine.ProjectileMovementComponent|SetHomingTargetComponent (Variables|Default|GetProjectileMovement) (Variables|/Game/BluePrint/BP_Player.BP_Player_C|GetStaticMesh _asbp_player)))))

(fn ConstructionScript
  (bind _projectilemovement (Variables|Default|GetProjectileMovement))
  (|CallParentFunction)
  (Transformation|SetWorldScale3D (Variables|Default|GetStaticMesh) (Variables|Default|GetScale))
  (bind _output_get (Variables|Default|SetMoveSpeed (Math|Random|RandomFloatinRange (Variables|Default|GetMinSpeed) (Variables|Default|GetMaxSpeed))))
  (bind _output_get_2 (Variables|/Script/Engine.ProjectileMovementComponent|SetMaxSpeed _projectilemovement _output_get))
  (Variables|/Script/Engine.ProjectileMovementComponent|SetInitialSpeed _projectilemovement _output_get_2))

(fn EnemyKilled
  (bind _returnvalue (Transformation|GetActorLocation))
  (bind _bp_gamemode (Variables|Default|GetBP_GameMode))
  (Default|SetScore _bp_gamemode (Variables|Default|GetEnemy%20score))
  (Default|PlayCameraShake _bp_gamemode 0 _returnvalue)
  (Audio|PlaySoundatLocation 0 _returnvalue "0, 0, 0" 1.0 1.0 0.0 0 0 0)
  (Actor|DestroyActor))